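; BP_TelekinesisObject is an object for a telekinesis mechanic that tracks and shows whether it is grabbed.
; Each call to its IsGrabbed event alternates through a FlipFlop, setting or clearing the IsGrabbed flag and swapping the static mesh material between GrabMaterial and MaterialInstance.
; It holds no movement logic, and its construction script only calls the parent.
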(event EventBeginPlay
  (|CallParentFunction) ; This node is disabled and will not be called.\nDrag off pins to build functionality.
)

(event EventIsGrabbed
  (Utilities|FlowControl|FlipFlop
    (:A
      (Variables|Default|SetIsGrabbed? true)
      (Rendering|Material|SetMaterial (Variables|Default|GetStaticMesh) 0 (Variables|Public|GetGrab%20Material)))
    (:B
      (Variables|Default|SetIsGrabbed? false)
      (Rendering|Material|SetMaterial (Variables|Default|GetStaticMesh) 0 (Variables|Default|GetMaterialInstance)))))

(event EventTick
  (params (DeltaSeconds :type Float%20%28single-precision%29)))

(event Collision|EventActorBeginOverlap
  (params (OtherActor :type Actor%20Object%20Reference)))

(fn ConstructionScript
  (|CallParentFunction))