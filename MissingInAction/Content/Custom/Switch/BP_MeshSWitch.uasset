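; Actor that toggles its static mesh between two world variants, MeshWorld0 and MeshWorld1, when its Switch event fires.
; Switch is ignored while the object is grabbed or mid-switch, otherwise it passes the World flag to SwitchMesh.
; SwitchMesh sets the mesh and IsEnable, flips World, then holds the switching lock for SwitchingTime.
; The disappear delay precedes the swap to MeshWorld1 but follows the swap to MeshWorld0.
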(event EventBeginPlay
  (|CallParentFunction) ; This node is disabled and will not be called.\nDrag off pins to build functionality.
)

(event Collision|EventActorBeginOverlap
  (params (OtherActor :type Actor%20Object%20Reference)))

(event EventTick
  (params (DeltaSeconds :type Float%20%28single-precision%29)))

(event EventSwitch
  (if (not (Variables|Default|GetIsGrabbed?))
    (if (not (Variables|Default|GetIsSwitching))
      (Utilities|SwitchMesh (Variables|Default|GetWorld)))))

(fn ConstructionScript
  (|CallParentFunction))