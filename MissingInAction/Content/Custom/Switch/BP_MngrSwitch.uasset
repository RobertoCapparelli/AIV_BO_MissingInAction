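; BP_MngrSwitch is a manager that toggles the level between two world states.
; On BeginPlay it caches all BP_BaseSwitch actors, the directional light and two post-process volumes taken by array index, disabling the second.
; Switch messages every cached switch actor on each call, even during cooldown.
; It then swaps light intensity and the active volume, gated by a flag that resets after a SwitchingTime delay.
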(event EventBeginPlay
  (bind _outactors (Actor|GetAllActorsOfClass "/Game/Custom/Switch/BP_BaseSwitch.BP_BaseSwitch_C"))
  (Variables|Default|SetComponentSwitch _outactors)
  (bind _returnvalue (Actor|GetActorOfClass "/Script/Engine.DirectionalLight"))
  (Variables|Default|SetDirectionalLight _returnvalue)
  (bind _outactors_2 (Actor|GetAllActorsOfClass "/Script/Engine.PostProcessVolume"))
  (Variables|Default|SetPostProcessWorld1 (Utilities|Array|Get(acopy) _outactors_2))
  (bind _output_get (Variables|Default|SetPostProcessWorld2 (Utilities|Array|Get(acopy) _outactors_2 1)))
  (Variables|/Script/Engine.PostProcessVolume|SetbEnabled _output_get false))

(event EventSwitch
  (Class|ISwitch|Switch(Message) (Variables|Default|GetComponentSwitch))
  (if (not (Variables|Default|GetIsSwitching))
    (Variables|Default|SetIsSwitching true)
    (if (Variables|Default|GetisEnable)
      (Rendering|Components|Light|SetIntensity (Variables|/Script/Engine.Light|GetLightComponent (Variables|Default|GetDirectionalLight)) (Variables|Default|GetIntensityWorld2))
      (Variables|/Script/Engine.PostProcessVolume|SetbEnabled (Variables|Default|GetPostProcessWorld1) false)
      (Variables|/Script/Engine.PostProcessVolume|SetbEnabled (Variables|Default|GetPostProcessWorld2) true)
      (else
        (Rendering|Components|Light|SetIntensity (Variables|/Script/Engine.Light|GetLightComponent (Variables|Default|GetDirectionalLight)) (Variables|Default|GetIntensityWorld1))
        (Variables|/Script/Engine.PostProcessVolume|SetbEnabled (Variables|Default|GetPostProcessWorld2) false)
        (Variables|/Script/Engine.PostProcessVolume|SetbEnabled (Variables|Default|GetPostProcessWorld1) true)))
    (Variables|Default|SetisEnable (not (Variables|Default|GetisEnable)))
    (Utilities|FlowControl|Delay (Variables|Default|GetSwitchingTime))
    (Variables|Default|SetIsSwitching false)))

(fn ConstructionScript)