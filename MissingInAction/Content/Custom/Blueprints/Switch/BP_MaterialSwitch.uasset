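; Switchable object that flips its static mesh between a solid world state and a pass-through ghost state.
; BeginPlay applies the ghost state if World is false, first caching the original material as a dynamic instance when MaterialWorld is unset.
; Switch, guarded by IsGrabbed and IsSwitching, runs SwitchMesh to swap material and Pawn collision response.
; Delays stagger collision and IsEnable changes and hold the switching lock.
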(event EventBeginPlay
  (Variables|Private|SetInitWorld (Variables|Public|GetWorld))
  (if (Variables|Public|GetWorld)
    (Variables|Private|SetIsEnable? true)
    (else
      (Variables|Public|GetMaterialWorld
        (:then
          _)
        (:else
          (bind _returnvalue (Rendering|Material|CreateDynamicMaterialInstance (Rendering|Material|GetMaterial (Variables|Default|GetStaticMesh) 0) "None" "None" :!class /Script/Engine.KismetMaterialLibrary))
          (Variables|Public|SetMaterialWorld _returnvalue)))
      (Rendering|Material|SetMaterial (Variables|Default|GetStaticMesh) 0 (Variables|Public|GetMaterialGhost))
      (Collision|SetCollisionResponsetoChannel (Variables|Default|GetStaticMesh) "ECC_Pawn" "ECR_Ignore"))))

(event EventSwitch
  (if (not (Variables|Private|GetIsGrabbed?))
    (if (not (Variables|Private|GetIsSwitching))
      (Utilities|SwitchMesh (Variables|Public|GetWorld)))))

(fn ConstructionScript)

(fn IsGrabbed
  (return))