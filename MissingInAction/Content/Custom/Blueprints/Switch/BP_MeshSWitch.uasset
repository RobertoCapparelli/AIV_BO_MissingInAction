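; Switchable world object that swaps its static mesh between two world variants and toggles an enabled flag to match.
; SwitchMesh picks the mesh from the World boolean, then flips it, delaying before the swap one way and after it the other.
; An IsSwitching guard blocks overlapping Switch calls, and IReset restores the initial World before switching again.
; The SwitchingTime cooldown delay is disconnected and never runs.
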(event EventBeginPlay
  (Variables|Default|SetInitWorld (Variables|Default|GetWorld))
  (|CallParentFunction)
  (Utilities|SwitchMesh (Variables|Default|GetWorld)))

(event EventIReset
  (Variables|Default|SetWorld (Variables|Default|GetInitWorld))
  (CallFunction|Switch))

(event EventSwitch
  (if (not (Variables|Default|GetIsSwitching))
    (Utilities|SwitchMesh (Variables|Default|GetWorld))))

(fn ConstructionScript
  (|CallParentFunction))