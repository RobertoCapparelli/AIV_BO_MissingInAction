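; Manager that toggles the level between two worlds, World0 and World1, changing their lighting and post-processing.
; BeginPlay caches all BP_AbstractSwitch actors and the DirectionalLight, then disables World0's post-process and spotlights.
; Switch messages those actors every call, then swaps light intensity, post-process volumes and spotlights, throttled by SwitchingTime.
; IReset re-runs Switch depending on a FlipFlop's state.
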(event EventBeginPlay
  (bind _outactors (Actor|GetAllActorsOfClass "/Game/Custom/Blueprints/Switch/BP_AbstractSwitch.BP_AbstractSwitch_C"))
  (Variables|Default|SetComponentSwitch _outactors)
  (bind _returnvalue (Actor|GetActorOfClass "/Script/Engine.DirectionalLight"))
  (Variables|Default|SetDirectionalLight _returnvalue)
  (Variables|/Script/Engine.PostProcessVolume|SetbEnabled (Variables|Default|GetPostProcessWorld0) false)
  (for _array_element (Variables|Default|GetLightsWorld0)
    (Development|SetHiddeninGame (Variables|/Script/Engine.SpotLight|GetSpotLightComponent _array_element) true false)))

(event EventIReset
  (if (stale _isa)
    (bind _isa (Utilities|FlowControl|FlipFlop)
      (:A
        _)
      (:B
        _))
    (Class|ISwitch|Switch(Message) (Variables|Default|GetComponentSwitch))
    (if (not (Variables|Default|GetIsSwitching))
      (Variables|Default|SetIsSwitching true)
      (if (Variables|Default|GetisEnable)
        (Rendering|Components|Light|SetIntensity (Variables|/Script/Engine.Light|GetLightComponent (Variables|Default|GetDirectionalLight)) (Variables|Default|GetIntensityDirectionalLightWorld1))
        (Variables|/Script/Engine.PostProcessVolume|SetbEnabled (Variables|Default|GetPostProcessWorld0) true)
        (Variables|/Script/Engine.PostProcessVolume|SetbEnabled (Variables|Default|GetPostProcessWorld1) false)
        (for _array_element (Variables|Default|GetLightsWorld0)
          (Development|SetHiddeninGame (Variables|/Script/Engine.SpotLight|GetSpotLightComponent _array_element) false false))
        (for _array_element_2 (Variables|Default|GetLightsWorld1)
          (Development|SetHiddeninGame (Variables|/Script/Engine.SpotLight|GetSpotLightComponent _array_element_2) true false))
        (else
          (Rendering|Components|Light|SetIntensity (Variables|/Script/Engine.Light|GetLightComponent (Variables|Default|GetDirectionalLight)) (Variables|Default|GetIntensityDirectionalLightWorld0))
          (Variables|/Script/Engine.PostProcessVolume|SetbEnabled (Variables|Default|GetPostProcessWorld1) true)
          (Variables|/Script/Engine.PostProcessVolume|SetbEnabled (Variables|Default|GetPostProcessWorld0) false)
          (for _array_element_3 (Variables|Default|GetLightsWorld1)
            (Development|SetHiddeninGame (Variables|/Script/Engine.SpotLight|GetSpotLightComponent _array_element_3) false false))
          (for _array_element_4 (Variables|Default|GetLightsWorld0)
            (Development|SetHiddeninGame (Variables|/Script/Engine.SpotLight|GetSpotLightComponent _array_element_4) true false))))
      (Variables|Default|SetisEnable (not (Variables|Default|GetisEnable)))
      (Utilities|FlowControl|Delay (Variables|Default|GetSwitchingTime))
      (Variables|Default|SetIsSwitching false))))

(event EventSwitch
  (bind _isa (Utilities|FlowControl|FlipFlop)
    (:A
      _)
    (:B
      _))
  (Class|ISwitch|Switch(Message) (Variables|Default|GetComponentSwitch))
  (if (not (Variables|Default|GetIsSwitching))
    (Variables|Default|SetIsSwitching true)
    (if (Variables|Default|GetisEnable)
      (Rendering|Components|Light|SetIntensity (Variables|/Script/Engine.Light|GetLightComponent (Variables|Default|GetDirectionalLight)) (Variables|Default|GetIntensityDirectionalLightWorld1))
      (Variables|/Script/Engine.PostProcessVolume|SetbEnabled (Variables|Default|GetPostProcessWorld0) true)
      (Variables|/Script/Engine.PostProcessVolume|SetbEnabled (Variables|Default|GetPostProcessWorld1) false)
      (for _array_element (Variables|Default|GetLightsWorld0)
        (Development|SetHiddeninGame (Variables|/Script/Engine.SpotLight|GetSpotLightComponent _array_element) false false))
      (for _array_element_2 (Variables|Default|GetLightsWorld1)
        (Development|SetHiddeninGame (Variables|/Script/Engine.SpotLight|GetSpotLightComponent _array_element_2) true false))
      (else
        (Rendering|Components|Light|SetIntensity (Variables|/Script/Engine.Light|GetLightComponent (Variables|Default|GetDirectionalLight)) (Variables|Default|GetIntensityDirectionalLightWorld0))
        (Variables|/Script/Engine.PostProcessVolume|SetbEnabled (Variables|Default|GetPostProcessWorld1) true)
        (Variables|/Script/Engine.PostProcessVolume|SetbEnabled (Variables|Default|GetPostProcessWorld0) false)
        (for _array_element_3 (Variables|Default|GetLightsWorld1)
          (Development|SetHiddeninGame (Variables|/Script/Engine.SpotLight|GetSpotLightComponent _array_element_3) false false))
        (for _array_element_4 (Variables|Default|GetLightsWorld0)
          (Development|SetHiddeninGame (Variables|/Script/Engine.SpotLight|GetSpotLightComponent _array_element_4) true false))))
    (Variables|Default|SetisEnable (not (Variables|Default|GetisEnable)))
    (Utilities|FlowControl|Delay (Variables|Default|GetSwitchingTime))
    (Variables|Default|SetIsSwitching false)))

(fn ConstructionScript)