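; Base switchable actor whose mesh toggles between a solid state and a ghost state, tracked by a World flag.
; BeginPlay caches the mesh's base material and applies the initial state.
; The Switch event runs SwitchMesh unless grabbed or mid-switch, swapping material and Pawn collision response with delays, then flipping World.
; IsGrabbed is an empty stub here, and only the Pawn channel changes, as the collision-enable toggles are disconnected.
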(event EventBeginPlay
  (bind _returnvalue (Rendering|Material|GetBaseMaterial (Rendering|Material|GetMaterial (Variables|Default|GetStaticMesh) 0)))
  (Variables|Private|SetMaterialInstance _returnvalue)
  (if (Variables|Public|GetWorld)
    (Variables|Private|SetIsEnable? true)
    (else
      (Rendering|Material|SetMaterial (Variables|Default|GetStaticMesh) 0 (Variables|Public|GetMaterialGhost))
      (Collision|SetCollisionResponsetoChannel (Variables|Default|GetStaticMesh) "ECC_Pawn" "ECR_Ignore"))))

(event EventSwitch
  (if (not (Variables|Private|GetIsGrabbed?))
    (if (not (Variables|Private|GetIsSwitching))
      (Utilities|SwitchMesh (Variables|Public|GetWorld)))))

(fn ConstructionScript)

(fn IsGrabbed
  (return))