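; Switchable mesh actor that starts hidden in game, becomes visible when Switch is called, and alternates its static mesh between two world states.
; BeginPlay and the Switch event pass the World flag to SwitchMesh, which picks the mesh, sets IsEnable and flips the flag.
; A delay precedes the swap to MeshWorld1 but follows the swap to MeshWorld0.
; IsSwitching blocks repeat switches until SwitchingTime has elapsed.
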(event EventBeginPlay
  (Rendering|SetActorHiddenInGame true)
  (|CallParentFunction)
  (Utilities|SwitchMesh (Variables|Default|GetWorld)))

(event EventSwitch
  (Rendering|SetActorHiddenInGame false)
  (if (not (Variables|Default|GetIsSwitching))
    (Utilities|SwitchMesh (Variables|Default|GetWorld))))

(fn ConstructionScript
  (|CallParentFunction))