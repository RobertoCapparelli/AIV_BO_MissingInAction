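; BP_Button is an overlap trigger that reveals a set of linked actors when the player touches it.
; On BeginPlay it hides every actor in ActorToActivate in game.
; Any overlap with its Box plays the button-press sound, but only actors tagged Player unhide the list, and nothing hides it again.
; TriggeredPlateMessage calls to other objects remain in the graph but never run.
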(event OnComponentBeginOverlap(Box)
  (params (OverlappedComponent :type Primitive%20Component%20Object%20Reference) (OtherActor :type Actor%20Object%20Reference) (OtherComp :type Primitive%20Component%20Object%20Reference) (OtherBodyIndex :type Integer) (bFromSweep :type Boolean) (SweepResult :type Hit%20Result%20Structure%20%28by%20ref%29))
  (Audio|PlaySoundatLocation "/Game/Custom/Sounds/Triggers/Portal_Button_pressed.Portal_Button_pressed" (Transformation|GetActorLocation) "0, 0, 0" 1.0 1.0 0.0 0 0 0 0)
  (if (Actor|ActorHasTag OtherActor "Player")
    (for _array_element (Variables|Default|GetActorToActivate)
      (Rendering|SetActorHiddenInGame _array_element false))))

(event EventBeginPlay
  (for _array_element (Variables|Default|GetActorToActivate)
    (Rendering|SetActorHiddenInGame _array_element true)))

(fn ConstructionScript)