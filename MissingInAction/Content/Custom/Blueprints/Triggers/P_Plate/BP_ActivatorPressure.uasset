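; BP_ActivatorPressure is a physics-simulated, color-coded object, apparently used to activate pressure plates.
; On BeginPlay it adds a Yellow, Green or Blue actor tag from TypeOfColor, then runs the parent logic.
; IReset restores the initial World value, calls Switch, then returns the actor to its initial transform, toggling mesh physics off during the move and back on afterward.
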(event EventBeginPlay
  (bind _self self)
  (bind _tags (Variables|Default|GetTags _self))
  (switch Utilities|FlowControl|Switch|SwitchonE_ColorPressurePlate (Variables|Default|GetTypeOfColor)
    (:NewEnumerator0
      (Utilities|Array|Add _tags "Yellow"))
    (:NewEnumerator1
      (Utilities|Array|Add _tags "Green"))
    (:NewEnumerator2
      (Utilities|Array|Add _tags "Blue")))
  (|CallParentFunction))

(event EventIReset
  (Variables|Default|SetWorld (Variables|Default|GetInitWorld))
  (CallFunction|Switch)
  (Physics|SetSimulatePhysics (Variables|Default|GetStaticMesh) false)
  (Transformation|SetActorTransform (Variables|Default|GetInitTransform))
  (Physics|SetSimulatePhysics (Variables|Default|GetStaticMesh) true))

(fn ConstructionScript)