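; Colour-matched pressure plate that only responds to overlapping actors tagged with the name of its TypeOfColor enum value.
; A timeline lowers the plate on overlap and reverses when the tagged actor leaves.
; Each time the timeline finishes, in either direction, it stores the direction and sends TriggeredPlateMessage to ObjectToActive.
; IReset reverses the plate from the end if the last stored direction was forward.
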(event OnComponentBeginOverlap(Box)
  (params (OverlappedComponent :type Primitive%20Component%20Object%20Reference) (OtherActor :type Actor%20Object%20Reference) (OtherComp :type Primitive%20Component%20Object%20Reference) (OtherBodyIndex :type Integer) (bFromSweep :type Boolean) (SweepResult :type Hit%20Result%20Structure%20%28by%20ref%29))
  (if (Actor|ActorHasTag OtherActor (Utilities|String|StringToName (Utilities|String|EnumtoString (Variables|Default|GetTypeOfColor))))
    (bind (_direction _alpha) (Timeline|PressurePlateAnimation Play)
      (:Update
        (Transformation|SetRelativeLocation (Variables|Default|GetPlate) (Math|Vector|MakeVector 0.0 0.0 (Math|Float|Lerp (Variables|Default|GetInitialPosition) (- (Variables|Default|GetInitialPosition) 9.0) _alpha)) false false))
      (:Finished
        (Variables|Default|SetDirection _direction)
        (Class|IPressurePlate|TriggeredPlate(Message) (Variables|Default|GetObjectToActive))))))

(event OnComponentEndOverlap(Box)
  (params (OverlappedComponent :type Primitive%20Component%20Object%20Reference) (OtherActor :type Actor%20Object%20Reference) (OtherComp :type Primitive%20Component%20Object%20Reference) (OtherBodyIndex :type Integer))
  (if (Actor|ActorHasTag (stale OnComponentBeginOverlap(Box) OtherActor) (Utilities|String|StringToName (Utilities|String|EnumtoString (Variables|Default|GetTypeOfColor))))
    (bind (_direction _alpha) (Timeline|PressurePlateAnimation Reverse)
      (:Update
        (Transformation|SetRelativeLocation (Variables|Default|GetPlate) (Math|Vector|MakeVector 0.0 0.0 (Math|Float|Lerp (Variables|Default|GetInitialPosition) (- (Variables|Default|GetInitialPosition) 9.0) _alpha)) false false))
      (:Finished
        (Variables|Default|SetDirection _direction)
        (Class|IPressurePlate|TriggeredPlate(Message) (Variables|Default|GetObjectToActive))))))

(event EventBeginPlay
  (Variables|Default|SetInitialPosition (.z (.location (Transformation|GetRelativeTransform (Variables|Default|GetPlate))))))

(event EventIReset
  (if (== (Variables|Default|GetDirection) 0)
    (bind (_direction _alpha) (Timeline|PressurePlateAnimation ReverseFromEnd)
      (:Update
        (Transformation|SetRelativeLocation (Variables|Default|GetPlate) (Math|Vector|MakeVector 0.0 0.0 (Math|Float|Lerp (Variables|Default|GetInitialPosition) (- (Variables|Default|GetInitialPosition) 9.0) _alpha)) false false))
      (:Finished
        (Variables|Default|SetDirection _direction)
        (Class|IPressurePlate|TriggeredPlate(Message) (Variables|Default|GetObjectToActive))))))

(fn ConstructionScript)