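; BP_ObjForTargetToss is an object for the target toss game, colored yellow, green or blue.
; On BeginPlay it adds the tag matching its TypeOfColor to both Tags and TagsNULL, then runs the parent BeginPlay and sets the TargetTossObj flag.
; The construction script only calls the parent, so all other behavior comes from the parent class.
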(event EventBeginPlay
  (bind _self self)
  (bind _tags (Variables|Default|GetTags _self))
  (switch Utilities|FlowControl|Switch|SwitchonE_ColorPressurePlate (Variables|Default|GetType%20Of%20Color)
    (:NewEnumerator0
      (Utilities|Array|Add _tags "Yellow")
      (Utilities|Array|Add (Variables|Default|GetTagsNULL) "Yellow"))
    (:NewEnumerator1
      (Utilities|Array|Add _tags "Green")
      (Utilities|Array|Add (Variables|Default|GetTagsNULL) "Green"))
    (:NewEnumerator2
      (Utilities|Array|Add _tags "Blue")
      (Utilities|Array|Add (Variables|Default|GetTagsNULL) "Blue")))
  (|CallParentFunction)
  (Variables|Default|SetbTargetTossObj true))

(fn ConstructionScript
  (|CallParentFunction))