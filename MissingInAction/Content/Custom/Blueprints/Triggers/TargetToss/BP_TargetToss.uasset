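; Toss target trigger that activates a linked object when an actor tagged "Toss" overlaps its box.
; A hit shifts the target along local Y and sends TriggeredPlateMessage to ObjectToActive; non-one-shot targets then reverse an offset timeline after a delay.
; OneShoot gates hits through a DoOnce, and IReset re-arms it and messages the object with a reset flag.
; On overlap end, tossed actors can optionally be hidden with collision disabled.
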(event OnComponentBeginOverlap(Box)
  (params (OverlappedComponent :type Primitive%20Component%20Object%20Reference) (OtherActor :type Actor%20Object%20Reference) (OtherComp :type Primitive%20Component%20Object%20Reference) (OtherBodyIndex :type Integer) (bFromSweep :type Boolean) (SweepResult :type Hit%20Result%20Structure%20%28by%20ref%29))
  (if (Actor|ActorHasTag OtherActor "Toss")
    (if (Variables|Default|GetOneShoot)
      (Utilities|FlowControl|DoOnce false
        (:Completed
          _)))
    (Transformation|SetRelativeLocation (Variables|Default|GetTarget) (Math|Vector|MakeVector 0.0 (- (Variables|Default|GetInitialPosition) 4.0) 0.0) false false)
    (Class|IPressurePlate|TriggeredPlate(Message) (Variables|Default|GetObject%20to%20Active) (Variables|Default|GetReset%20Call))
    (Variables|Default|SetReset%20Call false)
    (if (not (Variables|Default|GetOneShoot))
      (Utilities|FlowControl|Delay 1.0)
      (bind (_direction _alpha) (Timeline|alpha Reverse)
        (:Update
          (Transformation|SetRelativeLocation (Variables|Default|GetTarget) (Math|Vector|MakeVector 0.0 (Math|Float|Lerp (Variables|Default|GetInitialPosition) (- (Variables|Default|GetInitialPosition) 9.0) _alpha) 0.0) false false))
        (:Finished
          (Variables|Default|SetDirection _direction))))))

(event OnComponentEndOverlap(Box)
  (params (OverlappedComponent :type Primitive%20Component%20Object%20Reference) (OtherActor :type Actor%20Object%20Reference) (OtherComp :type Primitive%20Component%20Object%20Reference) (OtherBodyIndex :type Integer))
  (if (Actor|ActorHasTag (stale OnComponentBeginOverlap(Box) OtherActor) "Toss")
    (if (Variables|Default|GetDestroyOtherActorAfterActive)
      (Rendering|SetActorHiddenInGame (stale OnComponentBeginOverlap(Box) OtherActor) true)
      (Collision|SetActorEnableCollision (stale OnComponentBeginOverlap(Box) OtherActor) false))))

(event Custom|ResetOnce
  (Utilities|FlowControl|DoOnce false) ; enters at Reset
)

(event Custom|ResetTimeLine
  (Variables|Default|SetReset%20Call true)
  (Transformation|SetRelativeLocation (Variables|Default|GetTarget) (Math|Vector|MakeVector 0.0 (- (Variables|Default|GetInitialPosition) 4.0) 0.0) false false)
  (Class|IPressurePlate|TriggeredPlate(Message) (Variables|Default|GetObject%20to%20Active) (Variables|Default|GetReset%20Call))
  (Variables|Default|SetReset%20Call false)
  (if (not (Variables|Default|GetOneShoot))
    (Utilities|FlowControl|Delay 1.0)
    (bind (_direction _alpha) (Timeline|alpha Reverse)
      (:Update
        (Transformation|SetRelativeLocation (Variables|Default|GetTarget) (Math|Vector|MakeVector 0.0 (Math|Float|Lerp (Variables|Default|GetInitialPosition) (- (Variables|Default|GetInitialPosition) 9.0) _alpha) 0.0) false false))
      (:Finished
        (Variables|Default|SetDirection _direction)))))

(event EventBeginPlay
  (Variables|Default|SetInitialPosition (.y (.location (Transformation|GetRelativeTransform (Variables|Default|GetTarget))))))

(event EventIReset
  (CallFunction|ResetTimeLine)
  (CallFunction|ResetOnce))

(fn ConstructionScript)