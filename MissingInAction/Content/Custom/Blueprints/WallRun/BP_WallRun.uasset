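; BP_WallRun is a wall-run actor whose box trigger notifies the player on contact.
; When an actor tagged Player begins overlapping the box, it receives the IJumpFromWallMessage interface call with a false argument.
; The Switch event calls the parent's version, then sets the box's overlap-event generation to the inverse of World, so the trigger responds only while World is false.
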(event OnComponentBeginOverlap(Box)
  (params (OverlappedComponent :type Primitive%20Component%20Object%20Reference) (OtherActor :type Actor%20Object%20Reference) (OtherComp :type Primitive%20Component%20Object%20Reference) (OtherBodyIndex :type Integer) (bFromSweep :type Boolean) (SweepResult :type Hit%20Result%20Structure%20%28by%20ref%29))
  (if (Actor|ActorHasTag OtherActor "Player")
    (Class|IMovement|IJumpfromWall(Message) OtherActor false)))

(event EventBeginPlay
  (|CallParentFunction) ; This node is disabled and will not be called.\nDrag off pins to build functionality.
)

(event EventSwitch
  (|CallParentFunction)
  (Variables|/Script/Engine.PrimitiveComponent|SetbGenerateOverlapEvents (Variables|Default|GetBox) (not (Variables|Default|GetWorld))))

(fn ConstructionScript
  (|CallParentFunction))