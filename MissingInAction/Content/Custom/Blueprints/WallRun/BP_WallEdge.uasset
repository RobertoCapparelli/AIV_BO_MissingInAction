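; BP_WallEdge is a wall-run trigger that signals the player when a front-wall jump becomes available at an edge.
; On box overlap it compares the sweep impact normal to the player's forward vector within a tolerance, or exactly to its up vector.
; Matches send IJumpFrontWallMessage true, and leaving sends false.
; Inherited world switching toggles the box's overlap events and clears the player's jump state, while reset restores the initial world.
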(event OnComponentBeginOverlap(Box)
  (params (OverlappedComponent :type Primitive%20Component%20Object%20Reference) (OtherActor :type Actor%20Object%20Reference) (OtherComp :type Primitive%20Component%20Object%20Reference) (OtherBodyIndex :type Integer) (bFromSweep :type Boolean) (SweepResult :type Hit%20Result%20Structure%20%28by%20ref%29))
  (bind _output_get (Variables|Default|SetCanExit (and (Actor|ActorHasTag OtherActor "Player") (CallFunction|CalculateImpact (.impactnormal SweepResult)))))
  (if _output_get
    (Class|IMovement|IJumpFrontWall(Message) OtherActor true)))

(event OnComponentEndOverlap(Box)
  (params (OverlappedComponent :type Primitive%20Component%20Object%20Reference) (OtherActor :type Actor%20Object%20Reference) (OtherComp :type Primitive%20Component%20Object%20Reference) (OtherBodyIndex :type Integer))
  (if (and (Actor|ActorHasTag OtherActor "Player") (Variables|Default|GetCanExit))
    (Class|IMovement|IJumpFrontWall(Message) OtherActor false)))

(event EventBeginPlay
  (|CallParentFunction)
  (Variables|/Script/Engine.PrimitiveComponent|SetbGenerateOverlapEvents (Variables|Default|GetBox) (Variables|Default|GetWorld)))

(event EventSwitch
  (|CallParentFunction)
  (CallFunction|SetOverlapEvent)
  (Class|IMovement|IJumpFrontWall(Message) (Game|GetPlayerCharacter 0) false))

(event EventIReset
  (Variables|Default|SetWorld (Variables|Default|GetInitWorld))
  (CallFunction|Switch))

(fn ConstructionScript
  (|CallParentFunction))

(fn SetOverlapEvent
  (Variables|/Script/Engine.PrimitiveComponent|SetbGenerateOverlapEvents (Variables|Default|GetBox) (not (Variables|Default|GetWorld))))

(fn CalculateImpact
  (params (Result%20Impact :type Vector))
  (return (or (CallFunction|CalculateForwardImpact Result%20Impact) (CallFunction|CalculateUpImpact Result%20Impact))))

(fn CalculateForwardImpact
  (params (Result%20Impact :type Vector))
  (return (Utilities|Operators|EqualEqual Result%20Impact (Transformation|GetActorForwardVector (Game|GetPlayerCharacter 0)) (Variables|Default|GetSideTollerance))))

(fn CalculateUpImpact
  (params (Result%20Impact :type Vector))
  (return (Utilities|Operators|EqualEqual Result%20Impact (Transformation|GetActorUpVector (Game|GetPlayerCharacter 0)) 0.0)))