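; Climb component that lifts the player character up a wall and over its edge by stepping its location on a looping timer.
; Upper, gated by the externally set UppBox flag, disables the supplied movement component and starts the timer.
; Each tick runs a downward line trace, moving the character up while UppBox is set, then forward.
; When UppBox is clear and the trace hits a BP_WallEdge, movement resumes and the timer stops.
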(event Custom|Upper
  (if (Variables|Private|GetUppBox)
    (Components|Activation|SetActive (Variables|Private|GetCharacter%20Movement) false false)
    (bind _returnvalue (Utilities|Time|SetTimerbyEvent (delegate Custom|CustomEvent) (Variables|Public|GetUpperWallAnimationTime) true))
    (Variables|Private|SetUpper%20Animetion%20Timer _returnvalue)))

(event Custom|CustomEvent
  (bind (_start _end) (CallFunction|CalculateLineTraceVector))
  (bind (_outhits _returnvalue) (Collision|MultiLineTraceByChannel _start _end "TraceTypeQuery1" false 0 "Persistent"))
  (if _returnvalue
    (bind _array_element (Utilities|Array|ForEachLoopwithBreak _outhits)
      (:LoopBody
        (if (Variables|Private|GetUppBox)
          (CallFunction|MoveUp)
          (elif (CallFunction|IsCorrectHit (.hitactor _array_element))
            (Components|Activation|SetActive (Variables|Private|GetCharacter%20Movement) true false)
            (Utilities|Time|ClearandInvalidateTimerbyHandle (Variables|Private|GetUpper%20Animetion%20Timer))
            (else
              (CallFunction|MoveForward))))))
    (else
      (CallFunction|NotHitSequence))))

(event Custom|Init%20Component
  (params (Character%20Movement :type Character%20Movement%20Component%20Object%20Reference))
  ;[1 0 0] Initialize
  (Variables|Private|SetCharacter%20Movement Character%20Movement))

(event Custom|Set%20Upp%20Box
  (params (UppBox :type Boolean))
  (Variables|Private|SetUppBox UppBox))

(event Custom|Move%20Forward
  (Transformation|SetActorLocation (Variables|Private|GetCharacter) (CallFunction|CalculateFrontActorLocation) false false))

(event Custom|Move%20Up
  (Transformation|SetActorLocation (Variables|Private|GetCharacter) (CallFunction|CalculateUpActorLocation) true true))

(event Custom|Not%20Hit%20Sequence
  (if (Variables|Private|GetUppBox)
    (CallFunction|MoveUp)
    (else
      (CallFunction|MoveForward))))

(event EventBeginPlay
  ;[1 0 0] Initialize
  (Variables|Private|SetCharacter (Game|GetPlayerCharacter 0)))

(fn CalculateFrontActorLocation
  (bind _character (Variables|Private|GetCharacter))
  (return (+ (Transformation|GetActorForwardVector _character) (Transformation|GetActorLocation _character))))

(fn CalculateUpActorLocation
  (return (+ (Transformation|GetActorLocation (Variables|Private|GetCharacter)) "0.000000,0.000000,1.000000")))

(fn IsCorrectHit
  (params (Object :type Object%20Object%20Reference))
  (return (== (Utilities|GetClass Object) "/Game/Custom/Blueprints/WallRun/BP_WallEdge.BP_WallEdge_C")))

(fn CalculateLineTraceVector
  (bind _character (Variables|Private|GetCharacter))
  (bind _returnvalue (Transformation|GetActorLocation _character))
  (return _returnvalue (+ _returnvalue (* (Transformation|GetActorUpVector _character) -1e+02))))