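; Checkpoint actor that turns from red to green when the player overlaps it, sending an update-position message and, if flagged first, a remove-checkpoint message.
; On overlap it binds to the level's BP_Reset dispatcher and tells PreviewCheckpoint to unbind.
; Reset sends reset messages to its listed items, then cascades to NextCheckpoint, only when that list is non-empty.
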(event OnComponentBeginOverlap(Box)
  (params (OverlappedComponent :type Primitive%20Component%20Object%20Reference) (OtherActor :type Actor%20Object%20Reference) (OtherComp :type Primitive%20Component%20Object%20Reference) (OtherBodyIndex :type Integer) (bFromSweep :type Boolean) (SweepResult :type Hit%20Result%20Structure%20%28by%20ref%29))
  (if (Actor|ActorHasTag OtherActor "Player")
    (if (Variables|Public|GetIsFirstCheckpoint?)
      (Class|ICheckpoint|IRemoveCheckpoint(Message) OtherActor))
    (Class|ICheckpoint|IUpdatePosition(Message) OtherActor)
    (Rendering|Material|SetMaterial (Variables|Default|GetCube) 0 (Variables|Private|GetGreenMaterialInstance))
    (bind _resetter (Variables|Private|GetResetter)
      (:then
        (EventDispatchers|BindEventtoResetDispatcher _resetter (EventDispatchers|CreateEvent :!event Custom|Reset))
        (bind _previewcheckpoint (Variables|Public|GetPreviewCheckpoint)
          (:then
            (CallFunction|DisableReset _previewcheckpoint))
          (:else)))
      (:else))))

(event Custom|Reset
  (if (!= (Utilities|Array|Length (Variables|Public|GetItemToReset)) 0)
    (for _array_element (Variables|Public|GetItemToReset)
      (Class|IReset|IReset(Message) _array_element))
    (bind _nextcheckpoint (Variables|Public|GetNextCheckpoint)
      (:then
        (CallFunction|Reset _nextcheckpoint))
      (:else))))

(event Custom|Disable%20Reset
  (EventDispatchers|UnbindEventfromResetDispatcher (Variables|Private|GetResetter) (EventDispatchers|CreateEvent :!event Custom|Reset)))

(event EventBeginPlay
  (bind _returnvalue (Actor|GetActorOfClass "/Game/Custom/Blueprints/Reset/BP_Reset.BP_Reset_C"))
  (Variables|Private|SetResetter _returnvalue)
  (CallFunction|RedMaterial)
  (CallFunction|GreenMaterial)
  (Rendering|Material|SetMaterial (Variables|Default|GetCube) 0 (Variables|Private|GetRedMaterialInstance)))

(fn ConstructionScript)

(fn RedMaterial
  (bind _returnvalue (Rendering|Material|CreateDynamicMaterialInstance "/Game/Custom/Material/Red.Red" "None" "None" :!class /Script/Engine.KismetMaterialLibrary))
  (Variables|Private|SetRedMaterialInstance _returnvalue)
  (return))

(fn GreenMaterial
  (bind _returnvalue (Rendering|Material|CreateDynamicMaterialInstance "/Game/Custom/Material/Green.Green" "None" "None" :!class /Script/Engine.KismetMaterialLibrary))
  (Variables|Private|SetGreenMaterialInstance _returnvalue))