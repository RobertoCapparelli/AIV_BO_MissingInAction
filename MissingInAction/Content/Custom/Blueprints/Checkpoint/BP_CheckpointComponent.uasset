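; Actor component that stores a checkpoint transform for its owner and moves the owner back to it on demand.
; On BeginPlay it finds the BP_Checkpoint flagged as first and records the owner's starting transform; SavePosition later overwrites that transform.
; RestorePosition reapplies the saved transform and resets that first checkpoint if still valid, while RemoveCheckpoint clears the checkpoint reference.
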(event Custom|Save%20Position
  (Variables|Default|SetCheckpoint_Location (Transformation|GetActorTransform (Components|GetOwner))))

(event Custom|Restore%20Position
  (Transformation|SetActorTransform (Components|GetOwner) (Variables|Default|GetCheckpoint_Location))
  (bind _firstcheckpoint (Variables|Default|GetFirstCheckpoint)
    (:then
      (Default|Reset _firstcheckpoint))
    (:else)))

(event Custom|BreakLoop
  (Utilities|Array|ForEachLoopwithBreak (stale EventBeginPlay _outactors)) ; enters at Break
)

(event Custom|RemoveCheckpoint
  (Variables|Default|SetFirstCheckpoint 0))

(event EventBeginPlay
  (bind _outactors (Actor|GetAllActorsOfClass "/Game/Custom/Blueprints/Checkpoint/BP_Checkpoint.BP_Checkpoint_C"))
  (bind _array_element (Utilities|Array|ForEachLoopwithBreak _outactors)
    (:LoopBody
      (if (Variables|/Game/Custom/Blueprints/Checkpoint/BP_Checkpoint.BP_Checkpoint_C|GetIsFirstCheckpoint? _array_element)
        (Variables|Default|SetFirstCheckpoint _array_element)
        (CallFunction|BreakLoop)))
    (:Completed
      (Variables|Default|SetCheckpoint_Location (Transformation|GetActorTransform (Components|GetOwner))))))