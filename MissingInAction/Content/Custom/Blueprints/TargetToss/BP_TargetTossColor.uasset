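; Color-matched trigger plate for a target toss game, reacting to overlapping actors whose tag matches its color enum name.
; On a matching Box overlap, it shifts the Target mesh along local Y and sends TriggeredPlateMessage to ObjectToActive.
; When not flagged one-shot, it plays a timeline in reverse after a delay to lerp the Target back.
; Matching actors can optionally be hidden with collision disabled when the overlap ends.
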(event OnComponentBeginOverlap(Box)
  (params (OverlappedComponent :type Primitive%20Component%20Object%20Reference) (OtherActor :type Actor%20Object%20Reference) (OtherComp :type Primitive%20Component%20Object%20Reference) (OtherBodyIndex :type Integer) (bFromSweep :type Boolean) (SweepResult :type Hit%20Result%20Structure%20%28by%20ref%29))
  (if (Actor|ActorHasTag OtherActor (Utilities|String|StringToName (Utilities|String|EnumtoString (Variables|Default|GetTypeOfColor))))
    (if (Variables|Default|GetOneShoot)
      (Utilities|FlowControl|DoOnce false
        (:Completed
          _)))
    (Transformation|SetRelativeLocation (Variables|Default|GetTarget) (Math|Vector|MakeVector 0.0 (- (Variables|Default|GetInitialPosition) 4.0) 0.0) false false)
    (Class|IPressurePlate|TriggeredPlate(Message) (Variables|Default|GetObject%20to%20Active))
    (if (not (Variables|Default|GetOneShoot))
      (Utilities|FlowControl|Delay 1.0)
      (bind _alpha (Timeline|alpha Reverse)
        (:Update
          (Transformation|SetRelativeLocation (Variables|Default|GetTarget) (Math|Vector|MakeVector 0.0 (Math|Float|Lerp (Variables|Default|GetInitialPosition) (- (Variables|Default|GetInitialPosition) 9.0) _alpha) 0.0) false false))))))

(event OnComponentEndOverlap(Box)
  (params (OverlappedComponent :type Primitive%20Component%20Object%20Reference) (OtherActor :type Actor%20Object%20Reference) (OtherComp :type Primitive%20Component%20Object%20Reference) (OtherBodyIndex :type Integer))
  (if (Actor|ActorHasTag (stale OnComponentBeginOverlap(Box) OtherActor) (Utilities|String|StringToName (Utilities|String|EnumtoString (Variables|Default|GetTypeOfColor))))
    (if (Variables|Default|GetDestroyOtherActorAfterActive)
      (Rendering|SetActorHiddenInGame (stale OnComponentBeginOverlap(Box) OtherActor) true)
      (Collision|SetActorEnableCollision (stale OnComponentBeginOverlap(Box) OtherActor) false))))

(event EventBeginPlay
  (Variables|Default|SetInitialPosition (.y (.location (Transformation|GetRelativeTransform (Variables|Default|GetTarget))))))

(fn ConstructionScript)