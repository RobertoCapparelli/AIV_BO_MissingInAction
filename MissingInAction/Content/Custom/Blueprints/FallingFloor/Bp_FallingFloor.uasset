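; Falling floor tile that warns with a light and then drops after the player steps on it.
; When a Player-tagged actor overlaps the box, a timer turns the point light on, and a second timer then enables physics on the cube.
; An IReset event restores the cube's stored relative transform, stops physics and switches the light off.
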(event OnComponentBeginOverlap(Box)
  (params (OverlappedComponent :type Primitive%20Component%20Object%20Reference) (OtherActor :type Actor%20Object%20Reference) (OtherComp :type Primitive%20Component%20Object%20Reference) (OtherBodyIndex :type Integer) (bFromSweep :type Boolean) (SweepResult :type Hit%20Result%20Structure%20%28by%20ref%29))
  (if (Actor|ActorHasTag OtherActor "Player")
    (Utilities|Time|SetTimerbyEvent (EventDispatchers|CreateEvent :!event Custom|Warning) (Variables|Default|GetWarning%20Duration))))

(event Custom|Droptile
  (Physics|SetSimulatePhysics (Variables|Default|GetCube) true))

(event Custom|Warning
  (Rendering|Components|Light|SetIntensity (Variables|Default|GetPointLight) (Variables|Default|GetActive%20Intensity))
  (Utilities|Time|SetTimerbyEvent (EventDispatchers|CreateEvent :!event Custom|Droptile) (Variables|Default|GetAfter%20Warning%20Duration)))

(event EventBeginPlay
  (Rendering|Components|Light|SetIntensity (Variables|Default|GetPointLight) 0.0)
  (Variables|Default|SetRelativeTransform (Transformation|GetRelativeTransform (Variables|Default|GetCube))))

(event EventIReset
  (Physics|SetSimulatePhysics (Variables|Default|GetCube) false)
  (Transformation|SetRelativeTransform (Variables|Default|GetCube) (Variables|Default|GetRelativeTransform) false false)
  (Rendering|Components|Light|SetIntensity (Variables|Default|GetPointLight) 0.0))

(fn ConstructionScript)