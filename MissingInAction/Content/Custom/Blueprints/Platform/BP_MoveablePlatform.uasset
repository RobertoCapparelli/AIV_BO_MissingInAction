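; Moving platform that travels between waypoints placed as child components of its static mesh.
; BeginPlay caches their world transforms, then destroys those components.
; A single child gives an endless two-point swap; otherwise, after a start delay, MoveComponentTo steps ping-pong along the list, pausing between moves with an optional separate delay at the ends.
; Tick adds optional mesh spin, throttled by a time accumulator.
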(event Custom|MoveWithMultliplyPosition
  ;[1 1 1] move with multiplyPosition
  (Variables|Private|SetTempIterator (Variables|Private|GetIteratorNextPosition))
  (Components|MoveComponentTo (Variables|Default|GetDefaultSceneRoot) (Variables|Private|GetNextLocation) (Variables|Private|GetNextRotation) false false (Variables|Public|GetOverTime) true)
  (if (Variables|Private|GetIsMovingForward)
    ;;[1 1 1] iterator positive (i = 0, i > PlatformPosition.Lenght -1, i++)
    (bind _output_get (Variables|Private|SetIteratorNextPosition (+ (Variables|Private|GetIteratorNextPosition) 1)))
    (if (> _output_get (- (Utilities|Array|Length (Variables|Private|GetPlatformPositions)) 1))
      (Variables|Private|SetIsMovingForward false)
      (Variables|Private|SetIteratorNextPosition (- (Variables|Private|GetIteratorNextPosition) 2)))
    (else
      ;;[1 1 1] iterator negative (i = platform.lenght -1, i <= 0, i--)
      (bind _output_get_2 (Variables|Private|SetIteratorNextPosition (- (Variables|Private|GetIteratorNextPosition) 1)))
      (if (<= _output_get_2 0)
        (Variables|Private|SetIsMovingForward true))))
  (Variables|Private|SetNextLocation (Utilities|Array|Get(acopy) (Variables|Private|GetPlatformPositions) (Variables|Private|GetIteratorNextPosition)))
  (Variables|Private|SetNextRotation (Utilities|Array|Get(acopy) (Variables|Private|GetPlatformRotations) (Variables|Private|GetIteratorNextPosition)))
  (if (Variables|Public|GetStopAtFinishLap)
    (if (or (== (Variables|Private|GetTempIterator) 0) (== (- (Utilities|Array|Length (Variables|Private|GetPlatformPositions)) 1) (Variables|Private|GetTempIterator)))
      (Utilities|FlowControl|Delay (Variables|Public|GetEndDelay))
      (else
        (Utilities|FlowControl|Delay (Variables|Public|GetTimeStopPlatform) :!label _label)))
    (else
      (goto _label)))
  (CallFunction|MovewithMultliplyPosition))

(event Custom|MoveWith2Position
  ;[1 1 1] move with 2 position
  (Components|MoveComponentTo (Variables|Default|GetDefaultSceneRoot) (Variables|Private|GetNextLocation) (Variables|Private|GetNextRotation) false false (Variables|Public|GetOverTime) true)
  (Variables|Private|SetNextLocation (Variables|Private|GetCurrentLocation))
  (Variables|Private|SetCurrentLocation (Transformation|GetActorLocation))
  (Variables|Private|SetNextRotation (Variables|Private|GetCurrentRotation))
  (Variables|Private|SetCurrentRotation (Transformation|GetActorRotation))
  (Utilities|FlowControl|Delay (Variables|Public|GetTimeStopPlatform))
  (CallFunction|Movewith2Position))

(event EventTick
  (params (DeltaSeconds :type Float%20%28single-precision%29))
  ;[1 1 1] Rotation
  (if (Variables|Private|GetRotationRateValid)
    (bind _output_get (Variables|Private|SetTimeAccumulator (+ DeltaSeconds (Variables|Private|GetTimeAccumulator))))
    (if (>= _output_get 0.02)
      (Transformation|AddRelativeRotation (Variables|Default|GetStaticMesh) (Variables|Public|GetRotation%20Rate) false false)
      (Variables|Private|SetTimeAccumulator 0.0))))

(event EventBeginPlay
  (bind _staticmesh (Variables|Default|GetStaticMesh))
  (bind _children (Components|GetChildrenComponents _staticmesh true))
  ;[1 1 1] Start
  ;;[1 1 1] get all position for the platform after destroy all the mesh exept the original
  (|CallParentFunction)
  (Variables|Private|SetRotationRateValid (not (Utilities|Operators|EqualEqual :A (Variables|Public|GetRotation%20Rate))))
  (Utilities|Array|Add (Variables|Private|GetPlatformPositions) (Transformation|GetWorldLocation _staticmesh))
  (Utilities|Array|Add (Variables|Private|GetPlatformRotations) (Transformation|GetWorldRotation _staticmesh))
  (if (== (Utilities|Array|Length _children) 1)
    ;[1 1 1] if there's only 2 position
    (Variables|Private|SetNextLocation (Transformation|GetWorldLocation (Variables|Default|GetPosition2)))
    (Variables|Private|SetCurrentLocation (Transformation|GetWorldLocation (Variables|Default|GetStaticMesh)))
    (Variables|Private|SetNextRotation (Transformation|GetWorldRotation (Variables|Default|GetPosition2)))
    (Variables|Private|SetCurrentRotation (Transformation|GetWorldRotation (Variables|Default|GetStaticMesh)))
    (Components|DestroyComponent (Variables|Default|GetPosition2))
    (CallFunction|Movewith2Position)
    (else
      ;;;[1 1 1] If there's more position
      (for (_array_element _array_index) _children
        (Utilities|Array|Add (Variables|Private|GetPlatformPositions) (Transformation|GetWorldLocation _array_element))
        (Utilities|Array|Add (Variables|Private|GetPlatformRotations) (Transformation|GetWorldRotation _array_element))
        (if (> _array_index 0)
          (Variables|Private|SetCurrentLocation (Transformation|GetWorldLocation (Variables|Default|GetStaticMesh)))
          (Variables|Private|SetNextLocation (Transformation|GetWorldLocation (Variables|Default|GetPosition2)))
          (Variables|Private|SetCurrentRotation (Transformation|GetWorldRotation (Variables|Default|GetStaticMesh)))
          (Variables|Private|SetNextRotation (Transformation|GetWorldRotation (Variables|Default|GetPosition2)))))
      (bind _arrayelement (Utilities|Array|ReverseforEachLoop _children)
        (:LoopBody
          (Components|DestroyComponent _arrayelement))
        (:Completed
          ;;;[1 1 1] Start Loop
          (Utilities|FlowControl|Delay (Variables|Public|GetStartDelay))
          (CallFunction|MovewithMultliplyPosition))))))

(fn ConstructionScript
  (|CallParentFunction))