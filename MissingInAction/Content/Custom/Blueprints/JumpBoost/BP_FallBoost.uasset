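; BP_FallBoost gives the player a speed boost after landing lower than the jump's start point, paid from an energy pool shown on the HUD.
; Holding IA_Jump early in the fall arms it; once grounded, it raises walk speed and acceleration, draining energy initially and at whole-second hold times.
; Releasing restores acceleration, but not walk speed, and starts a looping timer that refills energy.
; PlayerLand is a leftover trace-based system.
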(event Custom|First%20Energy%20Reset
  ;[1 1 1] Boost Core
  (Utilities|FlowControl|DoOnce false) ; enters at Reset
)

(event Custom|Start%20Jump
  ;[1 1 1] Start Jump
  (Variables|Don'tTouch|SetStartLocation (Transformation|GetActorLocation (Game|GetPlayerCharacter 0)))
  (Utilities|Time|ClearandInvalidateTimerbyHandle (Variables|Don'tTouch|GetTimer))
  (CallFunction|SetDefaultAcceleration))

(event Custom|Player%20Land
  (bind _returnvalue (Game|GetPlayerCharacter 0))
  (bind _returnvalue_2 (Game|GetPlayerCharacter 0))
  (bind _startlocation (Variables|Don'tTouch|GetStartLocation))
  (bind _returnvalue_3 (Transformation|GetActorLocation _returnvalue))
  (bind _returnvalue_4 (Transformation|GetActorLocation _returnvalue_2))
  (bind _returnvalue_5 (- (.z _startlocation) (.z _returnvalue_3)))
  ;[1 1 1] OLD SYSTEM
  (bind _returnvalue_6 (Collision|LineTraceByChannel _returnvalue_4 (+ _returnvalue_4 (* (Math|Vector|GetUpVector (Variables|/Script/Engine.Character|GetCapsuleComponent _returnvalue_2)) -2e+02)) "TraceTypeQuery1" false 0 "Persistent"))
  (if (and (> _returnvalue_5 0.0) _returnvalue_6)
    _
    (else
      _))
  (Utilities|Time|ClearandInvalidateTimerbyHandle (Variables|Don'tTouch|GetTimer))
  (Development|PrintString (Utilities|String|ToString(Float) _returnvalue_5))
  (Development|PrintString "Hello"))

(event Custom|Start%20Reset%20Energy
  ;[1 1 1] Energy Restore System
  (bind _returnvalue (Utilities|Time|SetTimerbyEvent (delegate Custom|Restore%20%20Energy) 1.0 true))
  (Variables|Don'tTouch|SetTimer _returnvalue)
  (Variables|/Script/Engine.CharacterMovementComponent|SetMaxAcceleration (Variables|/Script/Engine.Character|GetCharacterMovement (Game|GetPlayerCharacter 0)) (Variables|Don'tTouch|GetStart%20Acceleration))
  (Variables|Don'tTouch|SetExecuted false)
  (Variables|Don'tTouch|SetIsBoost false)
  (CallFunction|FirstEnergyReset))

(event Custom|Restore%20%20Energy
  ;[1 1 1] Energy Restore System
  (if (> (+ (Variables|Settable|GetRestore%20Energy%20Ammount) (Variables|Don'tTouch|GetCurrent%20Energy)) (Variables|Settable|GetMax%20Energy))
    (Utilities|Time|ClearandInvalidateTimerbyHandle (Variables|Don'tTouch|GetTimer))
    (Variables|Don'tTouch|SetCurrent%20Energy (Variables|Settable|GetMax%20Energy))
    (CallFunction|SetWidgetEnergy)
    (else
      (Variables|Don'tTouch|SetCurrent%20Energy (+ (Variables|Settable|GetRestore%20Energy%20Ammount) (Variables|Don'tTouch|GetCurrent%20Energy)))
      (CallFunction|SetWidgetEnergy))))

(event Custom|Init
  (params (HUD :type WBP%20HUD%20Object%20Reference))
  ;[1 1 1] Init
  (Variables|Don'tTouch|SetCurrent%20Energy (Variables|Settable|GetMax%20Energy))
  (Variables|Don'tTouch|SetMin%20Energy (Variables|Settable|GetEnergy%20Cost))
  (Variables|Default|SetHUD HUD)
  (CallFunction|SetWidgetEnergy))

(event Input|EnhancedActionEvents|EnhancedInputActionIA_Jump
  (params (ActionValue :type Boolean) (ElapsedSeconds :type Float%20%28double-precision%29) (TriggeredSeconds :type Float%20%28double-precision%29) (InputAction :type Input%20Action%20Object%20Reference :default "/Game/FirstPerson/Input/Actions/IA_Jump.IA_Jump"))
  ;[1 1 1] Boost Core
  (:Ongoing
    (if (AI|Components|NavMovement|IsFalling (Variables|/Script/Engine.Character|GetCharacterMovement (Game|GetPlayerCharacter 0)))
      (if (CallFunction|CanExecuteJump ElapsedSeconds)
        (Variables|Don'tTouch|SetExecuted true)
        (else
          (Variables|Don'tTouch|SetExecuted false)))
      (elif (Math|Boolean|ANDBoolean (CallFunction|CheckHeightDifference) (Variables|Don'tTouch|GetExecuted) (CallFunction|CheckEnergy))
        (Utilities|FlowControl|Sequence
          (:then_0
            (Utilities|FlowControl|DoOnce false
              (:Completed
                (bind _output_get (CallFunction|ReduceEnergy))
                (Development|PrintString (Utilities|String|Append "REDUCE FIRST TIME " (Utilities|String|ToString(Float) _output_get))))))
          (:then_1
            (Variables|Don'tTouch|SetIsBoost true)
            (CallFunction|SetBoostParams)
            (if (CallFunction|CheckIntegerValues ElapsedSeconds)
              (CallFunction|ReduceEnergy)))))))
  (:Canceled
    (CallFunction|StartResetEnergy :!label _label))
  (:Completed
    (goto _label)))

(fn CheckHeightDifference
  (return (> (.z (Variables|Don'tTouch|GetStartLocation)) (.z (Transformation|GetActorLocation (Game|GetPlayerCharacter 0))))))

(fn CanExecuteJump
  (params (Time :type Float%20%28double-precision%29))
  (return (and (<= Time 0.5) (CallFunction|CheckEnergy))))

(fn SetDefaultAcceleration
  (Variables|Don'tTouch|SetStart%20Acceleration (Class|CharacterMovementComponent|GetMaxAcceleration (Variables|/Script/Engine.Character|GetCharacterMovement (Game|GetPlayerCharacter 0)))))

(fn CheckEnergy
  (return (>= (Variables|Don'tTouch|GetCurrent%20Energy) (Variables|Don'tTouch|GetMin%20Energy))))

(fn RoundFloatCustom
  (params (A :type Float%20%28double-precision%29))
  (return (* (Math|Float|Round (* A 1e+02)) 0.01)))

(fn ReduceEnergy
  (bind _output_get (Variables|Don'tTouch|SetCurrent%20Energy (- (Variables|Don'tTouch|GetCurrent%20Energy) (Variables|Settable|GetEnergy%20Cost))))
  (Default|SetEnergy (Variables|Default|GetHUD) (/ (Variables|Don'tTouch|GetCurrent%20Energy) (Variables|Settable|GetMax%20Energy)))
  (return _output_get))

(fn SetBoostParams
  (bind _returnvalue (Game|GetPlayerCharacter 0))
  (bind _charactermovement (Variables|/Script/Engine.Character|GetCharacterMovement _returnvalue))
  (Variables|/Script/Engine.CharacterMovementComponent|SetMaxWalkSpeed _charactermovement (Variables|Settable|GetBoost%20Max%20Walk%20Speed))
  (Variables|/Script/Engine.CharacterMovementComponent|SetMaxAcceleration _charactermovement (Variables|Settable|GetBoost%20Max%20Acceleration)))

(fn CheckIntegerValues
  (params (A :type Float%20%28double-precision%29))
  (return (< (Math|Float|%(Float) (CallFunction|RoundFloatCustom A) 1.0) 0.01)))

(fn SetWidgetEnergy
  (Default|SetEnergy (Variables|Default|GetHUD) (/ (Variables|Don'tTouch|GetCurrent%20Energy) (Variables|Settable|GetMax%20Energy))))