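; Physics object for a telekinesis mechanic, built on a parent that provides world switching.
; Each IsGrabbed event alternates grabbed and released states via a FlipFlop, changing the mesh's material and collision profile.
; BeginPlay and Switch set the actor's tags to either the saved set or TagsNULL depending on World.
; Respawn returns the mesh to its stored start location, briefly disabling physics simulation to move it.
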(event Custom|Respawn
  (Physics|SetSimulatePhysics (Variables|Default|GetStaticMesh) false)
  (Transformation|SetWorldLocation (Variables|Default|GetStaticMesh) (Variables|Default|GetInitPosition) false false)
  (Physics|SetSimulatePhysics (Variables|Default|GetStaticMesh) true))

(event EventBeginPlay
  (|CallParentFunction)
  (Variables|Default|SetTagsName (Variables|Default|GetTags self))
  (if (Variables|Default|GetWorld)
    (Variables|Default|SetTags self (Variables|Default|GetTagsName))
    (else
      (Variables|Default|SetTags self (Variables|Default|GetTagsNULL))))
  (Variables|Default|SetInitPosition (Transformation|GetWorldLocation (Variables|Default|GetStaticMesh))))

(event EventTick
  (params (DeltaSeconds :type Float%20%28single-precision%29)))

(event EventIsGrabbed
  (Utilities|FlowControl|FlipFlop
    (:A
      (Variables|Default|SetIsGrabbed? true)
      (Rendering|Material|SetMaterial (Variables|Default|GetStaticMesh) 0 (Variables|Public|GetMaterialGrab))
      (Collision|SetCollisionProfileName (Variables|Default|GetStaticMesh) "Telekinesis" true :!class /Script/Engine.PrimitiveComponent))
    (:B
      (Variables|Default|SetIsGrabbed? false)
      (Rendering|Material|SetMaterial (Variables|Default|GetStaticMesh) 0 (Variables|Default|GetMaterialWorld))
      (Collision|SetCollisionProfileName (Variables|Default|GetStaticMesh) "PhysicsActor" true :!class /Script/Engine.PrimitiveComponent))))

(event EventSwitch
  (|CallParentFunction)
  (if (Variables|Default|GetWorld)
    (Variables|Default|SetTags self (Variables|Default|GetTagsNULL))
    (else
      (Variables|Default|SetTags self (Variables|Default|GetTagsName)))))

(event Collision|EventActorBeginOverlap
  (params (OtherActor :type Actor%20Object%20Reference)))

(fn ConstructionScript
  (|CallParentFunction))