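; A platform that travels between its placed pose and a second pose each time it receives a grab event, if enabled.
; On BeginPlay it records the static mesh's world transform and that of the NextPosition marker component, then destroys the marker.
; Each grab toggles a FlipFlop that drives MoveComponentTo on the root, interpolating location and rotation to the other pose over OverTime.
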(event EventBeginPlay
  (bind _nextposition (Variables|Default|GetNextPosition))
  (bind _staticmesh (Variables|Default|GetStaticMesh))
  (|CallParentFunction)
  (Variables|Private|SetPos2 (Transformation|GetWorldLocation _nextposition))
  (Variables|Private|SetRot2 (Transformation|GetWorldRotation _nextposition))
  (Components|DestroyComponent (Variables|Default|GetNextPosition))
  (Variables|Private|SetPos1 (Transformation|GetWorldLocation _staticmesh))
  (Variables|Private|SetRot1 (Transformation|GetWorldRotation _staticmesh)))

(event EventIsGrabbed
  (bind _defaultsceneroot (Variables|Default|GetDefaultSceneRoot))
  (bind _over_time (Variables|Public|GetOver%20Time))
  (if (Variables|Default|GetIsEnable?)
    (Utilities|FlowControl|FlipFlop
      (:A
        (Components|MoveComponentTo _defaultsceneroot (Variables|Private|GetPos2) (Variables|Private|GetRot2) false false _over_time false))
      (:B
        (Components|MoveComponentTo _defaultsceneroot (Variables|Private|GetPos1) (Variables|Private|GetRot1) false false _over_time false)))))

(fn ConstructionScript
  (|CallParentFunction))