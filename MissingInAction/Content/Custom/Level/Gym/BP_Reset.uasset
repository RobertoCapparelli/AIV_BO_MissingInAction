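; BP_Reset is a gym level trigger that teleports any actor tagged Player to a preset location and rotation when it enters the box.
; Each overlap also calls a reset dispatcher after the teleport.
; A temporary hack, marked for removal, checks for the display name BP_Reset2 and, on that instance, spawns two target-toss objects at preset transforms and calls Switch on each.
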(event OnComponentBeginOverlap(Box)
  (params (OverlappedComponent :type Primitive%20Component%20Object%20Reference) (OtherActor :type Actor%20Object%20Reference) (OtherComp :type Primitive%20Component%20Object%20Reference) (OtherBodyIndex :type Integer) (bFromSweep :type Boolean) (SweepResult :type Hit%20Result%20Structure%20%28by%20ref%29))
  (if (Actor|ActorHasTag OtherActor "Player")
    (Transformation|SetActorLocationAndRotation OtherActor (Variables|Default|GetNew%20Location) (Variables|Default|GetNew%20Rotation) false true)
    (Default|CallResetDispatcher)
    ;[1 1 1] Remove ASAP
    (if (Utilities|Enum|Equal(Enum) (Utilities|GetDisplayName self) "BP_Reset2")
      (bind _returnvalue (Game|SpawnActorfromClass "/Game/Custom/Blueprints/TargetToss/BP_ObjForTargetToss.BP_ObjForTargetToss_C" (Variables|Default|GetSpawn1) "Undefined" "MultiplyWithRoot" 0 0))
      (Default|Switch _returnvalue)
      (bind _returnvalue_2 (Game|SpawnActorfromClass "/Game/Custom/Blueprints/TargetToss/BP_ObjForTargetToss.BP_ObjForTargetToss_C" (Variables|Default|GetSpawn2) "Undefined" "MultiplyWithRoot" 0 0))
      (Default|Switch _returnvalue_2))))

(fn ConstructionScript)